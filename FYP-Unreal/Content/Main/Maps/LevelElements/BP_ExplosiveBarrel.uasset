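; BP_ExplosiveBarrel is a level element that explodes after a delay when it takes any damage.
; Damage starts a sizzle sound at the barrel and activates its particle system for the TimetoExplode duration.
; It then stops the sound, spawns a BP_Explosion at the particle system's transform and destroys itself.
; The damage event has no guard against repeated hits during the fuse.
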(event Game|Damage|EventAnyDamage
  (params (Damage :type Float%20%28single-precision%29) (DamageType :type Damage%20Type%20Object%20Reference) (InstigatedBy :type Controller%20Object%20Reference) (DamageCauser :type Actor%20Object%20Reference))
  (bind _particlesystem (Variables|Default|GetParticleSystem))
  (bind _returnvalue (Audio|SpawnSoundatLocation (Variables|Default|GetSizzleSound) (Transformation|GetActorLocation) "0, 0, 0" 1.0 1.0 0.0 0 0))
  (Components|Activation|Activate _particlesystem false)
  (Utilities|FlowControl|Delay (Variables|Default|GetTimetoExplode))
  (Audio|Components|Audio|Stop _returnvalue)
  (Game|SpawnActorfromClass "/Game/Main/Entities/BaseClasses/BP_Explosion.BP_Explosion_C" (Transformation|GetWorldTransform _particlesystem) "AlwaysSpawn" "OverrideRootScale" 0 0)
  (Actor|DestroyActor))

(fn ConstructionScript)