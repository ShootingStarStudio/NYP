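; Interactable door that swings its movable mesh 90 degrees open or back closed.
; When opening, the player's position in the door's local space picks the swing direction, and the DoorMovement timeline drives the mesh's relative yaw.
; Interaction toggles Open through a DoOnce that resets when the timeline finishes, blocking input mid-swing.
; BeginPlay runs the same branch, animating the door to its initial state.
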(event EventBeginPlay
  (bind _movablestaticmesh (Variables|Default|GetMovableStaticMesh))
  (bind _relativerotation (Variables|/Script/Engine.SceneComponent|GetRelativeRotation _movablestaticmesh))
  (|CallParentFunction)
  (if (stale EventBPIInteract _output_get)
    (Math|Float|CompareFloat (Math|Float|Absolute(Float) (.yaw (Math|Conversions|RotationFromXVector (Math|Transform|InverseTransformLocation (Transformation|GetActorTransform) (Transformation|GetActorLocation (.PlayerRef (CallFunction|GetPlayerRef))))))) 9e+01
      (:>
        (Variables|Default|SetDirection 1 :!label _label)
        (bind _newtrack_0 (Timeline|DoorMovement PlayFromStart)
          (:Update
            (Transformation|SetRelativeRotation _movablestaticmesh (Math|Rotator|MakeRotator (.roll _relativerotation) (.pitch _relativerotation) (* _newtrack_0 9e+01 (Variables|Default|GetDirection))) false false))
          (:Finished
            (Utilities|FlowControl|DoOnce false) ; enters at Reset
          )))
      (:==
        (goto _label))
      (:<
        (Variables|Default|SetDirection -1)
        (Timeline|DoorMovement PlayFromStart)))
    (else
      (Timeline|DoorMovement ReverseFromEnd))))

(event EventBPIInteract
  (bind _movablestaticmesh (Variables|Default|GetMovableStaticMesh))
  (bind _relativerotation (Variables|/Script/Engine.SceneComponent|GetRelativeRotation _movablestaticmesh))
  (Utilities|FlowControl|DoOnce false :!label _label
    (:Completed
      (bind _output_get (Variables|Default|SetOpen (not (Variables|Default|GetOpen))))
      (if _output_get
        (Math|Float|CompareFloat (Math|Float|Absolute(Float) (.yaw (Math|Conversions|RotationFromXVector (Math|Transform|InverseTransformLocation (Transformation|GetActorTransform) (Transformation|GetActorLocation (.PlayerRef (CallFunction|GetPlayerRef))))))) 9e+01
          (:>
            (Variables|Default|SetDirection 1 :!label _label_2)
            (bind _newtrack_0 (Timeline|DoorMovement PlayFromStart)
              (:Update
                (Transformation|SetRelativeRotation _movablestaticmesh (Math|Rotator|MakeRotator (.roll _relativerotation) (.pitch _relativerotation) (* _newtrack_0 9e+01 (Variables|Default|GetDirection))) false false))
              (:Finished
                (goto _label Reset))))
          (:==
            (goto _label_2))
          (:<
            (Variables|Default|SetDirection -1)
            (Timeline|DoorMovement PlayFromStart)))
        (else
          (Timeline|DoorMovement ReverseFromEnd))))))

(fn ConstructionScript)