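; Fire extinguisher item that can be picked up into storage and sprayed to put out BP_Fire actors.
; Alt use runs the Niagara spray and enables a query-only capsule for a fixed delay, locking player movement meanwhile; primary use calls WeaponFire1.
; Capsule overlaps start dissipating a fire on entry and stop it on exit, printing debug messages.
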(event OnComponentBeginOverlap(Capsule)
  (params (OverlappedComponent :type Primitive%20Component%20Object%20Reference) (OtherActor :type Actor%20Object%20Reference) (OtherComp :type Primitive%20Component%20Object%20Reference) (OtherBodyIndex :type Integer) (bFromSweep :type Boolean) (SweepResult :type Hit%20Result%20Structure%20%28by%20ref%29))
  ;[1 1 1] Interaction With Fire
  (Utilities|IsValid OtherActor
    (:Is%20Valid
      (bind _asbp_fire (Utilities|Casting|CastToBP_Fire OtherActor))
      (Default|DissapateFire _asbp_fire)
      (Development|PrintString "Putting Out Fire"))))

(event OnComponentEndOverlap(Capsule)
  (params (OverlappedComponent :type Primitive%20Component%20Object%20Reference) (OtherActor :type Actor%20Object%20Reference) (OtherComp :type Primitive%20Component%20Object%20Reference) (OtherBodyIndex :type Integer))
  ;[1 1 1] Interaction With Fire
  (Utilities|IsValid OtherActor
    (:Is%20Valid
      (bind _asbp_fire (Utilities|Casting|CastToBP_Fire OtherActor))
      (Default|StopDissapting _asbp_fire)
      (Development|PrintString "Fire Paused"))))

(event EventBPIAltUse
  (bind _playerref (CallFunction|GetPlayerRef))
  ;[1 1 1] Use
  (Components|Activation|Activate (Variables|Default|GetNiagara) false)
  (Collision|SetCollisionEnabled (Variables|Default|GetCapsule) "QueryOnly")
  (Variables|/Game/Main/Player/IsometricOrbitCharacter.IsometricOrbitCharacter_C|SetCanMove? _playerref false)
  (Utilities|FlowControl|Delay 2.0)
  (Collision|SetCollisionEnabled (Variables|Default|GetCapsule) "NoCollision")
  (Components|Activation|Deactivate (Variables|Default|GetNiagara))
  (Variables|/Game/Main/Player/IsometricOrbitCharacter.IsometricOrbitCharacter_C|SetCanMove? _playerref true))

(event EventBPIUse
  ;[1 1 1] Use
  (CallFunction|WeaponFire1))

(event EventBPIInteract
  ;[1 1 1] Interact
  (Audio|SpawnSoundatLocation (Variables|Default|GetInteractSound) (Transformation|GetActorLocation) "0, 0, 0" 1.0 1.0 0.0 0 0)
  (CallFunction|StoreThisItem false (Variables|Default|GetItemStruct)))

(event EventBeginPlay
  ;[1 1 1] BeginPlay
  (|CallParentFunction)
  (Components|Activation|Deactivate (Variables|Default|GetNiagara))
  (Collision|SetCollisionEnabled (Variables|Default|GetCapsule) "NoCollision"))

(fn ConstructionScript)