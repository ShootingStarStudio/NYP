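; BP_Fire is a base fire hazard that costs the player stealth score if it is still present after an alarm delay.
; On BeginPlay it activates its particle system and, after the delay, calls StealthMinusScore on the player.
; DissapateFire runs a Timeline that rescales the collision sphere and destroys the fire when finished, while StopDissapting halts it.
; A sphere overlap passing a class check also destroys the actor.
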(event OnComponentBeginOverlap(Sphere)
  (params (OverlappedComponent :type Primitive%20Component%20Object%20Reference) (OtherActor :type Actor%20Object%20Reference) (OtherComp :type Primitive%20Component%20Object%20Reference) (OtherBodyIndex :type Integer) (bFromSweep :type Boolean) (SweepResult :type Hit%20Result%20Structure%20%28by%20ref%29))
  (if (Utilities|ClassIsChildOf (Utilities|GetClass OtherActor) 0)
    (Actor|DestroyActor)))

(event Custom|Dissapate%20Fire
  (bind _newtrack_0 (Timeline|Timeline Play)
    (:Update
      (Transformation|SetWorldScale3D (Variables|Default|GetSphere) (Math|Conversions|ToVector(Float) _newtrack_0)))
    (:Finished
      (Actor|DestroyActor))))

(event Custom|Stop%20Dissapting
  (bind _newtrack_0 (Timeline|Timeline Stop)
    (:Update
      (Transformation|SetWorldScale3D (Variables|Default|GetSphere) (Math|Conversions|ToVector(Float) _newtrack_0)))
    (:Finished
      (Actor|DestroyActor))))

(event EventBeginPlay
  (Components|Activation|Activate (Variables|Default|GetParticleSystem) false)
  (Utilities|FlowControl|Delay (Variables|Default|GetTimetoFireAlarm))
  (Default|StealthMinusScore (.PlayerRef (CallFunction|GetPlayerRef))))

(fn ConstructionScript)