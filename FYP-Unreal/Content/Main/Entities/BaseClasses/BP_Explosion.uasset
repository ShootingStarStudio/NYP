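; Base explosion actor that applies physics force, damage and effects at its location as soon as it spawns.
; On BeginPlay it fires a RadialForce impulse with strength and destructible damage scaled from ExplosionDamage, then spawns scaled particle and Niagara effects.
; One tick later it applies full, falloff-free radial damage within a separate DamageRadius and plays the sound, then destroys itself after a short delay.
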(event EventBeginPlay
  (bind _returnvalue (Transformation|GetActorTransform))
  (bind _explosiondamage (Variables|Default|GetExplosionDamage))
  (bind _effectscale (Variables|Default|GetEffectScale))
  (bind _radialforce (Variables|Default|GetRadialForce))
  (bind _returnvalue_2 (Math|Vector|MakeVector _effectscale _effectscale _effectscale))
  (bind _returnvalue_3 (* _explosiondamage 1e+03))
  (Variables|/Script/Engine.RadialForceComponent|SetRadius _radialforce (Variables|Default|GetForceRadius))
  (Variables|/Script/Engine.RadialForceComponent|SetDestructibleDamage _radialforce _returnvalue_3)
  (Variables|/Script/Engine.RadialForceComponent|SetImpulseStrength _radialforce _returnvalue_3)
  (Class|RadialForceComponent|FireImpulse _radialforce)
  (Effects|SpawnEmitteratLocation (Variables|Default|GetParticleEffect) (.location _returnvalue) (.rotation _returnvalue) _returnvalue_2 true "AutoRelease")
  (Niagara|SpawnSystematLocation (Variables|Default|GetExplosion_Niagara) (.location _returnvalue) (.rotation _returnvalue) _returnvalue_2 true true "AutoRelease")
  (Utilities|FlowControl|DelayUntilNextTick)
  (Game|Damage|ApplyRadialDamage (Variables|Default|GetExplosionDamage) (Transformation|GetActorLocation) (Variables|Default|GetDamageRadius) 0 0 self 0 true "ECC_Visibility")
  (Audio|SpawnSoundatLocation (Variables|Default|GetExplosionSound) (.location _returnvalue) "0, 0, 0" 1.0 1.0 0.0 0 0)
  (Utilities|FlowControl|Delay 1.0)
  (Actor|DestroyActor))

(fn ConstructionScript)