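; Base interactable actor that provides a prompt popup and a mesh highlight for interactions.
; UpdateInteract sets the popup's visibility and passes interact, pickup, eat, unlock and open flags to its W_Interactions widget, with a default reset at BeginPlay.
; While DisplayPopup is true, Tick sets the popup's world location to its cached starting relative location plus a vertical offset.
; UpdateHighlight toggles an overlay material on the static mesh.
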(event EventTick
  (params (DeltaSeconds :type Float%20%28single-precision%29))
  (Utilities|FlowControl|Sequence
    (:then_0
      (if (Variables|Default|GetDisplayPopup)
        (Transformation|SetWorldLocation (Variables|Default|GetInteractPopup) (+ (Variables|Default|GetWidget%20Loc) "0.000000,0.000000,50.000000") false false)))))

(event EventBeginPlay
  (Variables|Default|SetWidget%20Loc (Variables|/Script/Engine.SceneComponent|GetRelativeLocation (Variables|Default|GetInteractPopup)))
  (CallFunction|UpdateInteract false false false false false false))

(fn ConstructionScript)

(fn UpdateInteract
  (params (bNewVisibility :type Boolean) (IsInteract :type Boolean) (IsPickup :type Boolean) (IsEat :type Boolean) (IsUnlock :type Boolean) (IsOpen :type Boolean))
  (bind _interactpopup (Variables|Default|GetInteractPopup))
  (bind _asw_interactions (Utilities|Casting|CastToW_Interactions (UserInterface|GetWidget _interactpopup)))
  (Rendering|SetVisibility _interactpopup bNewVisibility false)
  (Variables|/Game/Main/UserInterface/Interactables/W_Interactions.W_Interactions_C|SetIsInteract _asw_interactions IsInteract)
  (Variables|/Game/Main/UserInterface/Interactables/W_Interactions.W_Interactions_C|SetIsPickup _asw_interactions IsPickup)
  (Variables|/Game/Main/UserInterface/Interactables/W_Interactions.W_Interactions_C|SetIsEat _asw_interactions IsEat)
  (Variables|/Game/Main/UserInterface/Interactables/W_Interactions.W_Interactions_C|SetIsUnlock _asw_interactions IsUnlock)
  (Variables|/Game/Main/UserInterface/Interactables/W_Interactions.W_Interactions_C|SetIsOpen _asw_interactions IsOpen)
  (Default|UpdateData _asw_interactions))

(fn UpdateHighlight
  (params (State :type Boolean))
  (bind _staticmesh (Variables|Default|GetStaticMesh))
  (if State
    (Rendering|Material|SetOverlayMaterial _staticmesh (Variables|Default|GetOverlayMaterial) :!class /Script/Engine.MeshComponent)
    (else
      (Rendering|Material|SetOverlayMaterial _staticmesh 0 :!class /Script/Engine.MeshComponent))))