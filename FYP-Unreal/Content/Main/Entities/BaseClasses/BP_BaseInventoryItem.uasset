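; Base inventory item actor that the player can store and drop, filling its data from a data table row on BeginPlay.
; A sphere collider toggles highlight and interaction when the IsometricOrbitCharacter overlaps it.
; Storing uses either the player's rock inventory for pre-allocated slots or the general inventory, which also updates the UI.
; Dropping detaches the mesh, teleports the actor and restores physics, collision and visibility through a shared state toggle.
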(event OnComponentBeginOverlap(SphereCollider)
  (params (OverlappedComponent :type Primitive%20Component%20Object%20Reference) (OtherActor :type Actor%20Object%20Reference) (OtherComp :type Primitive%20Component%20Object%20Reference) (OtherBodyIndex :type Integer) (bFromSweep :type Boolean) (SweepResult :type Hit%20Result%20Structure%20%28by%20ref%29))
  (Utilities|Casting|CastToIsometricOrbitCharacter OtherActor)
  (CallFunction|UpdateHighlight true)
  (CallFunction|UpdateInteract true false false false false false))

(event OnComponentEndOverlap(SphereCollider)
  (params (OverlappedComponent :type Primitive%20Component%20Object%20Reference) (OtherActor :type Actor%20Object%20Reference) (OtherComp :type Primitive%20Component%20Object%20Reference) (OtherBodyIndex :type Integer))
  (Utilities|Casting|CastToIsometricOrbitCharacter OtherActor)
  (CallFunction|UpdateHighlight false)
  (CallFunction|UpdateInteract false false false false false false))

(event Custom|Store%20This%20Item
  (params (PreAllocated%20Slot :type Boolean) (ItemData :type S%20Inventory%20Item%20Structure))
  (bind _playerref (CallFunction|GetPlayerRef))
  (bind _self self)
  (if PreAllocated%20Slot
    (bind _success (Default|AddRocktoInventory _playerref _self))
    (if _success
      _)
    (else
      (bind _success_2 (Default|AddItemtoInventory _playerref _self))
      (if _success_2
        (Default|AddItemtoUIInventory (Variables|/Game/Main/Player/IsometricOrbitCharacter.IsometricOrbitCharacter_C|GetWInventory%20Reference _playerref) ItemData)))))

(event Custom|Drop%20This%20Item
  (params (Drop%20Location :type Vector))
  (Transformation|DetachFromComponent (Variables|Default|GetStaticMesh) "KeepWorld" "KeepWorld" "KeepWorld" true)
  (Transformation|SetActorLocation Drop%20Location false true)
  (CallFunction|UpdatePhysicsState true))

(event EventBeginPlay
  (bind _ac_itemdatacomponent (Variables|Default|GetAC_ItemDataComponent))
  (bind _itemid (Variables|/Game/Main/UserInterface/Inventory/AC_ItemDataComponent.AC_ItemDataComponent_C|GetItemID _ac_itemdatacomponent))
  (Variables|Default|SetPlayerRef (.PlayerRef (CallFunction|GetPlayerRef)))
  (bind _returnvalue (Utilities|GetDataTableRow (.datatable _itemid) (.rowname _itemid))
    (:then
      (bind _output_get (Variables|Default|SetItemStruct _returnvalue))
      (Variables|Default|SetItemStruct (Utilities|Struct|MakeS_InventoryItem self (.classref _output_get) (.name _output_get) (.icon _output_get) (.watchimage _output_get) (.description _output_get) (.weapontype _output_get) (.equipsound _output_get) (.pickupsound _output_get) (.destroyedsound _output_get))))))

(fn ConstructionScript)

(fn UpdatePhysicsState
  (params (State :type Boolean))
  (bind _staticmesh (Variables|Default|GetStaticMesh))
  (bind _sphere_collider (Variables|Default|GetSphere%20Collider))
  (if State
    (Physics|SetSimulatePhysics _staticmesh true)
    (Collision|SetCollisionEnabled _staticmesh "QueryAndPhysics")
    (Collision|SetCollisionEnabled _sphere_collider "QueryOnly")
    (CallFunction|UpdateVisualState true)
    (else
      (Physics|SetSimulatePhysics _staticmesh false)
      (Collision|SetCollisionEnabled _staticmesh "NoCollision")
      (Collision|SetCollisionEnabled _sphere_collider "NoCollision")
      (CallFunction|UpdateVisualState false))))

(fn UpdateVisualState
  (params (Can%20See :type Boolean))
  (Rendering|SetActorHiddenInGame (not Can%20See)))