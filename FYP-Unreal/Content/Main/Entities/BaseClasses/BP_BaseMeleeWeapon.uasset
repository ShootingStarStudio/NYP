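; Base melee weapon whose fire and ADS inputs both trigger the same swing, with a random knife sound and a guard against overlapping attacks.
; A looping timer at frame-delta intervals runs a short forward capsule trace from EmitterLoc, starting after an impact delay and stopping when the attack duration ends.
; Hit actors take damage and join the trace's ignore list, limiting each to one hit per swing until the list resets.
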(event Custom|AttackCall
  (bind _emitterloc (Variables|Default|GetEmitterLoc))
  (bind _returnvalue (Transformation|GetWorldLocation _emitterloc))
  (bind (_outhit _returnvalue_2) (Collision|CapsuleTraceByChannel _returnvalue (+ _returnvalue (* (Math|Vector|GetForwardVector _emitterloc) 4e+01)) 2e+01 1e+01 "TraceTypeQuery1" false (Variables|Default|GetHitActor) "None" true "(R=0.000000,G=0.409570,B=1.000000,A=1.000000)" "(R=0.000000,G=1.000000,B=0.337707,A=1.000000)" 0.4))
  (if _returnvalue_2
    (Game|Damage|ApplyDamage (.HitActor (Collision|BreakHitResult _outhit)) (Variables|Default|GetDamage) 0 self)
    (Utilities|Array|AddUnique (Variables|Default|GetHitActor) (.HitActor (Collision|BreakHitResult _outhit)))))

(event Custom|ADS_Override
  (bind _returnvalue (Transformation|GetActorLocation))
  (if (not (Variables|Default|GetisMeleeAttacking))
    (Variables|Default|SetisMeleeAttacking true)
    (switch int (Math|Random|RandomInteger 3)
      (:Default
        (Audio|SpawnSoundatLocation "/Game/Main/SoundEffects/NewSoundStuffs/Knife_Swing_3.Knife_Swing_3" _returnvalue "0, 0, 0" 1.0 1.0 0.0 0 0 :!label _label))
      (:0
        (Audio|SpawnSoundatLocation "/Game/Main/SoundEffects/NewSoundStuffs/Knife_Swing_1.Knife_Swing_1" _returnvalue "0, 0, 0" 1.0 1.0 0.0 0 0))
      (:1
        (Audio|SpawnSoundatLocation "/Game/Main/SoundEffects/NewSoundStuffs/Knife_Swing_2.Knife_Swing_2" _returnvalue "0, 0, 0" 1.0 1.0 0.0 0 0))
      (:2
        (goto _label)))
    (bind _returnvalue_2 (Utilities|Time|SetTimerbyEvent (delegate Custom|AttackCall) (Utilities|Time|GetWorldDeltaSeconds) true (Variables|Default|GetDelayUntilImpact)))
    (Utilities|FlowControl|Delay (Variables|Default|GetAttackDuration))
    (Utilities|Time|ClearandInvalidateTimerbyHandle _returnvalue_2)
    (Variables|Default|SetisMeleeAttacking false)
    (Variables|Default|SetHitActor (Variables|Default|GetActorsToIgnore))))

(event Custom|WeaponFire_1
  (bind _returnvalue (Transformation|GetActorLocation))
  (if (not (Variables|Default|GetisMeleeAttacking))
    (Variables|Default|SetisMeleeAttacking true)
    (switch int (Math|Random|RandomInteger 3)
      (:Default
        (Audio|SpawnSoundatLocation "/Game/Main/SoundEffects/NewSoundStuffs/Knife_Swing_3.Knife_Swing_3" _returnvalue "0, 0, 0" 1.0 1.0 0.0 0 0 :!label _label))
      (:0
        (Audio|SpawnSoundatLocation "/Game/Main/SoundEffects/NewSoundStuffs/Knife_Swing_1.Knife_Swing_1" _returnvalue "0, 0, 0" 1.0 1.0 0.0 0 0))
      (:1
        (Audio|SpawnSoundatLocation "/Game/Main/SoundEffects/NewSoundStuffs/Knife_Swing_2.Knife_Swing_2" _returnvalue "0, 0, 0" 1.0 1.0 0.0 0 0))
      (:2
        (goto _label)))
    (bind _returnvalue_2 (Utilities|Time|SetTimerbyEvent (delegate Custom|AttackCall) (Utilities|Time|GetWorldDeltaSeconds) true (Variables|Default|GetDelayUntilImpact)))
    (Utilities|FlowControl|Delay (Variables|Default|GetAttackDuration))
    (Utilities|Time|ClearandInvalidateTimerbyHandle _returnvalue_2)
    (Variables|Default|SetisMeleeAttacking false)
    (Variables|Default|SetHitActor (Variables|Default|GetActorsToIgnore))))

(fn ConstructionScript)