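; Base objective actor that, when the player overlaps it, activates every BP_Goal in the level and clears the objective.
; The overlap event loops over all goals, calling GoalActivated on each.
; Inside that same loop it also marks the player's objectives widget clear, plays the clear sound, and destroys itself after a one-tick delay, so widget and sound calls repeat per goal.
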(event Collision|EventActorBeginOverlap
  (params (OtherActor :type Actor%20Object%20Reference))
  (bind _playerref (CallFunction|GetPlayerRef))
  ;[1 1 1] Overlap With Player
  (Utilities|IsValid OtherActor
    (:Is%20Valid
      (if (== OtherActor _playerref)
        (bind _outactors (Actor|GetAllActorsOfClass "/Game/Main/Maps/LevelElements/BP_Goal.BP_Goal_C"))
        (bind _array_element (Utilities|Array|ForEachLoopwithBreak _outactors)
          (:LoopBody
            (Utilities|IsValid _array_element
              (:Is%20Valid
                (Default|GoalActivated _array_element)
                (Default|SetClear (Variables|/Game/Main/Player/IsometricOrbitCharacter.IsometricOrbitCharacter_C|GetWObjectives%20Reference _playerref))
                (Audio|SpawnSound2D "/Game/Main/SoundEffects/Objective_Clear.Objective_Clear" 1.0 1.0 0.0 0)
                (Utilities|FlowControl|DelayUntilNextTick)
                (Actor|DestroyActor))))
          (:Completed
            (Development|PrintString "All Goal Active")))))))

(fn ConstructionScript)