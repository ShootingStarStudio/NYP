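; BP_SoundWave is an expanding sound detection actor that lets enemies hear it.
; It starts at zero scale and grows uniformly each Tick at MaxRadius divided by GrowthTime, then destroys itself on reaching MaxRadius.
; Any BP_Enemy it overlaps while growing gets OnHear called with the wave as argument.
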(event Collision|EventActorBeginOverlap
  (params (OtherActor :type Actor%20Object%20Reference))
  (if (Utilities|ClassIsChildOf (Utilities|GetClass OtherActor) "/Game/Main/Entities/Enemies/FSM/BP_Enemy.BP_Enemy_C")
    (bind _asbp_enemy (Utilities|Casting|CastToBP_Enemy OtherActor))
    (Default|OnHear _asbp_enemy self)))

(event EventTick
  (params (DeltaSeconds :type Float%20%28single-precision%29))
  (bind _returnvalue (Transformation|GetActorScale3D))
  (bind _maxradius (Variables|Default|GetMaxRadius))
  (bind _growthrate (Variables|Default|GetGrowthRate))
  (bind _returnvalue_2 (* DeltaSeconds _growthrate))
  (bind _returnvalue_3 (+ _returnvalue_2 (.x _returnvalue)))
  (bind _returnvalue_4 (Math|Float|Clamp(Float) _returnvalue_3 0.0 _maxradius))
  (Transformation|SetActorScale3D (Math|Vector|MakeVector _returnvalue_4 _returnvalue_4 _returnvalue_4))
  (Math|Float|CompareFloat _returnvalue_4 _maxradius
    (:>
      _)
    (:==
      _))
  (Actor|DestroyActor))

(event EventBeginPlay
  (Transformation|SetActorScale3D "0, 0, 0")
  (Variables|Default|SetGrowthRate (/ (Variables|Default|GetMaxRadius) (Variables|Default|GetGrowthTime))))

(fn ConstructionScript)